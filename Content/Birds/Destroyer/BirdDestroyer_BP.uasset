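; BirdDestroyer_BP is a trigger wall that removes birds that reach it and counts them as missed.
; When a Bird_MasterBP overlaps its box, it calls BirdDestroyed on the bird, destroys it, and calls MissedBird on the PlayerBP cached at BeginPlay.
; The construction script scales the box from Width and Height into a thin slab, so its size can be set per instance.
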(event OnComponentBeginOverlap(Box)
  (params (OverlappedComponent :type Primitive%20Component%20Object%20Reference) (OtherActor :type Actor%20Object%20Reference) (OtherComp :type Primitive%20Component%20Object%20Reference) (OtherBodyIndex :type Integer) (bFromSweep :type Boolean) (SweepResult :type Hit%20Result%20Structure%20%28by%20ref%29))
  (bind _asbird_master_bp (Utilities|Casting|CastToBird_MasterBP OtherActor))
  (Default|BirdDestroyed _asbird_master_bp)
  (Actor|DestroyActor _asbird_master_bp)
  (Default|MissedBird (Variables|Default|GetPlayerBPRef)))

(event EventBeginPlay
  (bind _asplayer_bp (Utilities|Casting|CastToPlayerBP (Game|Player|GetPlayerPawn 0)))
  (Variables|Default|SetPlayerBPRef _asplayer_bp))

(fn ConstructionScript
  (Transformation|SetWorldScale3D (Variables|Default|GetBox) (Math|Vector|MakeVector (Variables|Default|GetWidth) 0.1 (Variables|Default|GetHeight))))