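; Base bird target that registers with the player's bird total on spawn and gets knocked out by a thrown stone.
; The first overlap with a live StoneProjectile_BP adds its points to the stone's score, notifies player and stone, and destroys the bird after a delay.
; The bird mesh attaches to the stone's pivot, optionally sticking to the stone first, with pitch-randomized hit sounds and a multiplier-pitched bonus sound.
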(event OnComponentBeginOverlap(BirdCollision)
  (params (OverlappedComponent :type Primitive%20Component%20Object%20Reference) (OtherActor :type Actor%20Object%20Reference) (OtherComp :type Primitive%20Component%20Object%20Reference) (OtherBodyIndex :type Integer) (bFromSweep :type Boolean) (SweepResult :type Hit%20Result%20Structure%20%28by%20ref%29))
  (bind _birdhurtsound (Variables|Default|GetBirdHurtSound))
  ;[1 1 1] Collision
  (bind _asstone_projectile_bp (Utilities|Casting|CastToStoneProjectile_BP OtherActor))
  (bind _output_get (Variables|Refs|SetStoneProjectileRef _asstone_projectile_bp))
  (Variables|/Game/Projectile/StoneProjectile_BP.StoneProjectile_BP_C|SetBirdBPRef _output_get self)
  (if (not (Variables|/Game/Projectile/StoneProjectile_BP.StoneProjectile_BP_C|GetbDeadStone _output_get))
    (Utilities|FlowControl|DoOnce false
      (:Completed
        (CallFunction|BirdHIt)
        (Default|HitBird _output_get)
        (if (Variables|Default|GetbStickToStone)
          (Transformation|AttachComponentToComponent (Variables|Default|GetSK_BIrd) (Variables|/Game/Projectile/StoneProjectile_BP.StoneProjectile_BP_C|GetStone _output_get) "None" "KeepRelative" "KeepRelative" "KeepRelative" true)
          (Utilities|FlowControl|Sequence
            (:then_0
              (Utilities|FlowControl|Delay 0.5)
              (Transformation|AttachComponentToComponent (Variables|Default|GetSK_BIrd) (Variables|/Game/Projectile/StoneProjectile_BP.StoneProjectile_BP_C|GetBirdPivot _output_get) "None" "KeepRelative" "KeepRelative" "KeepRelative" true))
            (:then_1
              (Audio|PlaySoundatLocation (Utilities|Array|Get(acopy) (Variables|Default|GetBirdHitSoundEffects) (Math|Random|RandomIntegerinRange 0 (Utilities|Array|Length (Variables|Default|GetBirdHitSoundEffects)))) (Transformation|GetWorldLocation (Variables|/Game/Projectile/StoneProjectile_BP.StoneProjectile_BP_C|GetBirdPivot _output_get)) "0, 0, 0" 1.0 (Math|Random|RandomFloatinRange 0.8 1.2) 0.0 0 0 0 :!label _label)
              (Utilities|IsValid _birdhurtsound
                (:Is%20Valid
                  (Audio|PlaySoundatLocation _birdhurtsound "0, 0, 0" "0, 0, 0" 1.0 (Math|Random|RandomFloatinRange 1.0 1.4) 0.0 0 0 0)))))
          (else
            (Transformation|AttachComponentToComponent (Variables|Default|GetSK_BIrd) (Variables|/Game/Projectile/StoneProjectile_BP.StoneProjectile_BP_C|GetBirdPivot _output_get) "None" "KeepRelative" "KeepRelative" "KeepRelative" true)
            (goto _label)))))))

(event Custom|ShowBonus
  ;[1 1 1] Bonus 2 birds 1 stone
  (Utilities|FlowControl|Delay 0.2)
  (if (Variables|Default|GetbGotBonus)
    (CallFunction|PlayBonusSound)))

(event Custom|PlayBonusSound
  ;[1 1 1] Bonus 2 birds 1 stone
  (Audio|PlaySoundatLocation "/Game/Audio/SoundEffects/Success/Success01_Cue.Success01_Cue" (Transformation|GetWorldLocation (Variables|Default|GetRoot)) "0, 0, 0" 1.0 (* (Variables|/Game/Projectile/StoneProjectile_BP.StoneProjectile_BP_C|GetCurrentMultiplier (Variables|Refs|GetStoneProjectileRef)) 0.5) 0.0 0 0 0))

(event Custom|KillBird
  ;[1 1 1] Kill Bird
  (Collision|SetCollisionEnabled (Variables|Default|GetBirdCollision) "NoCollision")
  (Utilities|FlowControl|Delay 2.0)
  (Actor|DestroyActor))

(event EventBeginPlay
  ;[1 1 1] Begin Play
  (bind _asplayer_bp (Utilities|Casting|CastToPlayerBP (Game|Player|GetPlayerPawn 0)))
  (bind _output_get (Variables|Default|SetPlayerBPRef _asplayer_bp))
  (Math|Integer|IncrementInt (Variables|/Game/Player/PlayerBP.PlayerBP_C|GetTotalBirds _output_get)))

(event Collision|EventActorBeginOverlap
  (params (OtherActor :type Actor%20Object%20Reference)))

(fn ConstructionScript)

(fn BirdHIt
  (bind _stoneprojectileref (Variables|Refs|GetStoneProjectileRef))
  (Variables|Default|SetbBirdHit true)
  (Default|HitBird (Variables|Default|GetPlayerBPRef))
  (CallFunction|ShowBonus)
  (CallFunction|KillBird)
  (Variables|/Game/Projectile/StoneProjectile_BP.StoneProjectile_BP_C|SetCurrentScore _stoneprojectileref (+ (Variables|/Game/Projectile/StoneProjectile_BP.StoneProjectile_BP_C|GetCurrentScore _stoneprojectileref) (Variables|Default|GetBirdPointValue))))

(fn BirdDestroyed)