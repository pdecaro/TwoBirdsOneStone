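; Golden Goose bird, a child Blueprint that flies a fixed waypoint path across the level after a short spawn delay.
; FromLeft picks the order through the five GoldenGooseSpawnRef targets, 05 to 01 or 01 to 05, finishing at SpawnLeftEnd or SpawnRightEnd.
; Each leg snaps the root toward the next point, then moves it with a timed, latent MoveComponentTo.
; BirdHIt extends the parent's hit handling with a looping hit animation.
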(event EventBeginPlay
  (bind _goldengoosespawnref (Variables|Default|GetGoldenGooseSpawnRef))
  (bind _root (Variables|Default|GetRoot))
  (bind _root_2 (Variables|Default|GetRoot))
  (bind _goldengoosespawnref_2 (Variables|Default|GetGoldenGooseSpawnRef))
  (bind _goldengoosespawnref_3 (Variables|Default|GetGoldenGooseSpawnRef))
  (bind _root_3 (Variables|Default|GetRoot))
  (bind _goldengoosespawnref_4 (Variables|Default|GetGoldenGooseSpawnRef))
  (bind _root_4 (Variables|Default|GetRoot))
  (bind _goldengoosespawnref_5 (Variables|Default|GetGoldenGooseSpawnRef))
  (bind _goldengoosespawnref_6 (Variables|Default|GetGoldenGooseSpawnRef))
  (bind _goldengoosespawnref_7 (Variables|Default|GetGoldenGooseSpawnRef))
  (bind _goldengoosespawnref_8 (Variables|Default|GetGoldenGooseSpawnRef))
  (bind _goldengoosespawnref_9 (Variables|Default|GetGoldenGooseSpawnRef))
  (bind _goldengoosespawnref_10 (Variables|Default|GetGoldenGooseSpawnRef))
  (bind _goldengoosespawnref_11 (Variables|Default|GetGoldenGooseSpawnRef))
  (bind _root_5 (Variables|Default|GetRoot))
  (bind _root_6 (Variables|Default|GetRoot))
  (bind _root_7 (Variables|Default|GetRoot))
  (bind _root_8 (Variables|Default|GetRoot))
  (bind _root_9 (Variables|Default|GetRoot))
  (bind _root_10 (Variables|Default|GetRoot))
  (bind _root_11 (Variables|Default|GetRoot))
  (bind _root_12 (Variables|Default|GetRoot))
  (bind _goldengoosespawnref_12 (Variables|Default|GetGoldenGooseSpawnRef))
  (bind _returnvalue (Transformation|GetWorldLocation _root_10))
  (bind _returnvalue_2 (Transformation|GetWorldLocation _root_11))
  (bind _returnvalue_3 (Transformation|GetWorldLocation _root_12))
  (bind _returnvalue_4 (Transformation|GetWorldLocation _root))
  (bind _returnvalue_5 (Transformation|GetWorldLocation _root_2))
  (bind _returnvalue_6 (Transformation|GetWorldLocation _root_3))
  (bind _returnvalue_7 (Transformation|GetWorldLocation _root_4))
  (bind _returnvalue_8 (Transformation|GetWorldLocation _root_5))
  (bind _returnvalue_9 (Transformation|GetWorldLocation _root_6))
  (bind _returnvalue_10 (Transformation|GetWorldLocation _root_7))
  (bind _returnvalue_11 (Transformation|GetWorldLocation _root_8))
  (bind _returnvalue_12 (Transformation|GetWorldLocation _root_9))
  (bind _target03 (Variables|/Game/Birds/Spawners/GoldenGoose_Spawner.GoldenGoose_Spawner_C|GetTarget03 _goldengoosespawnref_2))
  (bind _target05 (Variables|/Game/Birds/Spawners/GoldenGoose_Spawner.GoldenGoose_Spawner_C|GetTarget05 _goldengoosespawnref_5))
  (bind _target04 (Variables|/Game/Birds/Spawners/GoldenGoose_Spawner.GoldenGoose_Spawner_C|GetTarget04 _goldengoosespawnref_6))
  (bind _target03_2 (Variables|/Game/Birds/Spawners/GoldenGoose_Spawner.GoldenGoose_Spawner_C|GetTarget03 _goldengoosespawnref_7))
  (bind _target02 (Variables|/Game/Birds/Spawners/GoldenGoose_Spawner.GoldenGoose_Spawner_C|GetTarget02 _goldengoosespawnref_8))
  (bind _target01 (Variables|/Game/Birds/Spawners/GoldenGoose_Spawner.GoldenGoose_Spawner_C|GetTarget01 _goldengoosespawnref_9))
  (bind _spawnleftend (Variables|/Game/Birds/Spawners/GoldenGoose_Spawner.GoldenGoose_Spawner_C|GetSpawnLeftEnd _goldengoosespawnref_11))
  (bind _target01_2 (Variables|/Game/Birds/Spawners/GoldenGoose_Spawner.GoldenGoose_Spawner_C|GetTarget01 _goldengoosespawnref_10))
  (bind _target02_2 (Variables|/Game/Birds/Spawners/GoldenGoose_Spawner.GoldenGoose_Spawner_C|GetTarget02 _goldengoosespawnref_12))
  (bind _target04_2 (Variables|/Game/Birds/Spawners/GoldenGoose_Spawner.GoldenGoose_Spawner_C|GetTarget04 _goldengoosespawnref_3))
  (bind _target05_2 (Variables|/Game/Birds/Spawners/GoldenGoose_Spawner.GoldenGoose_Spawner_C|GetTarget05 _goldengoosespawnref_4))
  (bind _spawnrightend (Variables|/Game/Birds/Spawners/GoldenGoose_Spawner.GoldenGoose_Spawner_C|GetSpawnRightEnd _goldengoosespawnref))
  (bind _returnvalue_13 (Transformation|GetWorldLocation _target03))
  (bind _returnvalue_14 (Transformation|GetWorldLocation _target04_2))
  (bind _returnvalue_15 (Transformation|GetWorldLocation _target05_2))
  (bind _returnvalue_16 (Transformation|GetWorldLocation _spawnrightend))
  (bind _returnvalue_17 (Transformation|GetWorldLocation _target05))
  (bind _returnvalue_18 (Transformation|GetWorldLocation _target04))
  (bind _returnvalue_19 (Transformation|GetWorldLocation _target03_2))
  (bind _returnvalue_20 (Transformation|GetWorldLocation _target02))
  (bind _returnvalue_21 (Transformation|GetWorldLocation _target01))
  (bind _returnvalue_22 (Transformation|GetWorldLocation _spawnleftend))
  (bind _returnvalue_23 (Transformation|GetWorldLocation _target01_2))
  (bind _returnvalue_24 (Transformation|GetWorldLocation _target02_2))
  (bind _returnvalue_25 (Math|Rotator|FindLookatRotation _returnvalue _returnvalue_13))
  (bind _returnvalue_26 (Math|Rotator|FindLookatRotation _returnvalue_2 _returnvalue_14))
  (bind _returnvalue_27 (Math|Rotator|FindLookatRotation _returnvalue_3 _returnvalue_15))
  (bind _returnvalue_28 (Math|Rotator|FindLookatRotation _returnvalue_4 _returnvalue_16))
  (bind _returnvalue_29 (Math|Rotator|FindLookatRotation _returnvalue_5 _returnvalue_17))
  (bind _returnvalue_30 (Math|Rotator|FindLookatRotation _returnvalue_6 _returnvalue_18))
  (bind _returnvalue_31 (Math|Rotator|FindLookatRotation _returnvalue_7 _returnvalue_19))
  (bind _returnvalue_32 (Math|Rotator|FindLookatRotation _returnvalue_8 _returnvalue_20))
  (bind _returnvalue_33 (Math|Rotator|FindLookatRotation _returnvalue_9 _returnvalue_21))
  (bind _returnvalue_34 (Math|Rotator|FindLookatRotation _returnvalue_10 _returnvalue_22))
  (bind _returnvalue_35 (Math|Rotator|FindLookatRotation _returnvalue_11 _returnvalue_23))
  (bind _returnvalue_36 (Math|Rotator|FindLookatRotation _returnvalue_12 _returnvalue_24))
  (|CallParentFunction)
  (Utilities|FlowControl|Delay 0.5)
  (if (Variables|Default|GetbFromLeft)
    (Transformation|SetRelativeRotation _root_2 _returnvalue_29 false false)
    (Components|MoveComponentTo (Variables|Default|GetRoot) (.location (Transformation|GetWorldTransform _target05)) _returnvalue_29 false false 1.5 true)
    (Transformation|SetRelativeRotation (Variables|Default|GetRoot) _returnvalue_30 false false)
    (Components|MoveComponentTo (Variables|Default|GetRoot) (.location (Transformation|GetWorldTransform _target04)) _returnvalue_30 false false 3.0 true)
    (Transformation|SetRelativeRotation (Variables|Default|GetRoot) _returnvalue_31 false false)
    (Components|MoveComponentTo (Variables|Default|GetRoot) (.location (Transformation|GetWorldTransform _target03_2)) _returnvalue_31 false false 1.5 false)
    (Transformation|SetRelativeRotation (Variables|Default|GetRoot) _returnvalue_32 false false)
    (Components|MoveComponentTo (Variables|Default|GetRoot) (.location (Transformation|GetWorldTransform _target02)) _returnvalue_32 false false 1.5 false)
    (Transformation|SetRelativeRotation (Variables|Default|GetRoot) _returnvalue_33 false false)
    (Components|MoveComponentTo (Variables|Default|GetRoot) (.location (Transformation|GetWorldTransform _target01)) _returnvalue_33 false false 3.0 false)
    (Transformation|SetRelativeRotation (Variables|Default|GetRoot) _returnvalue_34 false false)
    (Components|MoveComponentTo (Variables|Default|GetRoot) (.location (Transformation|GetWorldTransform _spawnleftend)) _returnvalue_34 false false 1.5 false)
    (else
      (Transformation|SetRelativeRotation (Variables|Default|GetRoot) _returnvalue_35 false false)
      (Components|MoveComponentTo (Variables|Default|GetRoot) (.location (Transformation|GetWorldTransform _target01_2)) _returnvalue_35 false false 1.5 false)
      (Transformation|SetRelativeRotation (Variables|Default|GetRoot) _returnvalue_36 false false)
      (Components|MoveComponentTo (Variables|Default|GetRoot) (.location (Transformation|GetWorldTransform _target02_2)) _returnvalue_36 false false 3.0 false)
      (Transformation|SetRelativeRotation (Variables|Default|GetRoot) _returnvalue_25 false false)
      (Components|MoveComponentTo (Variables|Default|GetRoot) (.location (Transformation|GetWorldTransform _target03)) _returnvalue_25 false false 1.5 false)
      (Transformation|SetRelativeRotation (Variables|Default|GetRoot) _returnvalue_26 false false)
      (Components|MoveComponentTo (Variables|Default|GetRoot) (.location (Transformation|GetWorldTransform _target04_2)) _returnvalue_26 false false 1.5 false)
      (Transformation|SetRelativeRotation (Variables|Default|GetRoot) _returnvalue_27 false false)
      (Components|MoveComponentTo (Variables|Default|GetRoot) (.location (Transformation|GetWorldTransform _target05_2)) _returnvalue_27 false false 3.0 false)
      (Transformation|SetRelativeRotation (Variables|Default|GetRoot) _returnvalue_28 false false)
      (Components|MoveComponentTo (Variables|Default|GetRoot) (.location (Transformation|GetWorldTransform _spawnrightend)) _returnvalue_28 false false 1.5 false))))

(event Collision|EventActorBeginOverlap
  (params (OtherActor :type Actor%20Object%20Reference))
  (|CallParentFunction OtherActor) ; This node is disabled and will not be called.\nDrag off pins to build functionality.
)

(event EventTick
  (params (DeltaSeconds :type Float%20%28single-precision%29)))

(fn ConstructionScript
  (|CallParentFunction))

(fn BirdHIt
  (|CallParentFunction)
  (Components|Animation|PlayAnimation (Variables|Default|GetSK_BIrd) "/Game/Models/Birds/GoldenGoose/Animations/GoldenGoose_Hit_anim.GoldenGoose_Hit_anim" true))