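; Flying duck Blueprint, a hittable bird that crosses the scene left to right or right to left while honking.
; After BeginPlay, MoveComponentTo carries the root along Y by TravelDistance, with Speed shortening the duration.
; A looping random delay plays honks with varied sound and pitch, and a Flapping timeline bobs the placeholder vertically.
; The BirdHIt override stops flapping, silences further honks, randomly rotates the mesh and releases detached feather effects.
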(event Custom|MoveLeftToRight
  (bind _root (Variables|Default|GetRoot))
  (bind _relativelocation (Variables|/Script/Engine.SceneComponent|GetRelativeLocation _root))
  ;[1 1 1] Movement
  ;;[1 1 1] Move Left To Right
  (Components|MoveComponentTo _root (Math|Vector|MakeVector (.x _relativelocation) (* (Variables|Default|GetTravelDistance) 1.0) (.z _relativelocation)) "0, 0, 0" false false (- 3e+01 (* (Variables|Default|GetSpeed) 2.0)) false))

(event Custom|Hit
  (bind _placeholder (Variables|Default|GetPlaceHolder))
  (bind _relativelocation (Variables|/Script/Engine.SceneComponent|GetRelativeLocation _placeholder))
  ;[1 1 1] Bird Hit
  (bind _flap (Timeline|Flapping Stop)
    (:Update
      (Transformation|SetRelativeLocation _placeholder (Math|Vector|MakeVector (.x _relativelocation) (.y _relativelocation) _flap) false false))))

(event Custom|MoveRightToLeft
  (bind _root (Variables|Default|GetRoot))
  (bind _relativelocation (Variables|/Script/Engine.SceneComponent|GetRelativeLocation _root))
  ;[1 1 1] Movement
  ;;[1 1 1] Move Right To Left
  (Components|MoveComponentTo _root (Math|Vector|MakeVector (.x _relativelocation) (* (Variables|Default|GetTravelDistance) -1.0) (.z _relativelocation)) "0, 0, 0" false false (- 3e+01 (* (Variables|Default|GetSpeed) 2.0)) false))

(event Custom|ReleaseFeathers
  (bind _duckfeathers (Variables|Default|GetDuckFeathers))
  (Transformation|DetachFromComponent _duckfeathers "KeepWorld" "KeepWorld" "KeepRelative" true)
  (Components|Activation|Activate _duckfeathers false))

(event Custom|Honk
  ;[1 1 1] Honk
  (if (not (Variables|Default|GetbHit))
    (Audio|PlaySoundatLocation (Utilities|Array|Get(acopy) (Variables|Default|GetHonkingSounds) (Math|Random|RandomIntegerinRange 0 3)) (Transformation|GetWorldLocation (Variables|Default|GetRoot)) "0, 0, 0" 1.0 (Math|Random|RandomFloatinRange 0.8 1.2) 0.0 0 0 0)))

(event Custom|PlayHonkSounds
  ;[1 1 1] Honk
  (Utilities|FlowControl|Delay (Math|Random|RandomFloatinRange 0.75 2.0) :!label _label)
  (CallFunction|Honk)
  (goto _label))

(event EventBeginPlay
  ;[1 1 1] Begin Play
  (|CallParentFunction)
  (Utilities|FlowControl|Delay 0.2)
  (if (Variables|Default|GetbLeftToRight)
    (CallFunction|MoveLefttoRight)
    (else
      (CallFunction|MoveRighttoLeft)))
  (CallFunction|PlayHonkSounds))

(event Collision|EventActorBeginOverlap
  (params (OtherActor :type Actor%20Object%20Reference))
  (|CallParentFunction OtherActor) ; This node is disabled and will not be called.\nDrag off pins to build functionality.
)

(event EventTick
  (params (DeltaSeconds :type Float%20%28single-precision%29))
  (|CallParentFunction DeltaSeconds) ; This node is disabled and will not be called.\nDrag off pins to build functionality.
)

(fn ConstructionScript
  (|CallParentFunction))

(fn BirdHIt
  (bind _returnvalue (Math|Random|RandomFloatinRange -2e+01 2e+01))
  (|CallParentFunction)
  (CallFunction|Hit)
  (Variables|Default|SetbHit true)
  (Transformation|SetRelativeRotation (Variables|Default|GetSK_BIrd) (Math|Rotator|MakeRotator _returnvalue _returnvalue (Math|Random|RandomFloatinRange -2e+02 -1.6e+02)) false false)
  (CallFunction|ReleaseFeathers))