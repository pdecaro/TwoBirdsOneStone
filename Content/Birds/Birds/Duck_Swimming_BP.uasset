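; Swimming duck bird actor that moves along a track's spline and reacts to being hit.
; Shortly after BeginPlay, an active duck starts a timeline scaled by Duration that sets its location and rotation along the spline, or destroys itself if the track reference is invalid.
; The BirdHIt override stops the ripple effect, randomly rotates the skeletal mesh and detaches the feather effect in world space before activating it.
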(event Custom|MoveDuck
  (Components|Timeline|SetPlayRate (Variables|Default|GetDuckMover) (/ 1.0 (Variables|Default|GetDuration)))
  (bind _alpha (Timeline|DuckMover Play)
    (:Update
      (Variables|Default|SetAlpha _alpha)
      (Transformation|SetActorLocationAndRotation (Spline|GetLocationatDistanceAlongSpline (Variables|/Game/Birds/Paths/Track_BP.Track_BP_C|GetPathSpline (Variables|Default|GetTrack_BPRef)) (Math|Float|Lerp 0.0 (Spline|GetSplineLength (Variables|/Game/Birds/Paths/Track_BP.Track_BP_C|GetPathSpline (Variables|Default|GetTrack_BPRef))) (Variables|Default|GetAlpha)) "World") (Spline|GetRotationatDistanceAlongSpline (Variables|/Game/Birds/Paths/Track_BP.Track_BP_C|GetPathSpline (Variables|Default|GetTrack_BPRef)) (Math|Float|Lerp 0.0 (Spline|GetSplineLength (Variables|/Game/Birds/Paths/Track_BP.Track_BP_C|GetPathSpline (Variables|Default|GetTrack_BPRef))) (Variables|Default|GetAlpha)) "World")))))

(event Custom|ReleaseFeathers
  (bind _duckfeathers (Variables|Default|GetDuckFeathers))
  (Transformation|DetachFromComponent _duckfeathers "KeepWorld" "KeepWorld" "KeepRelative" true)
  (Components|Activation|Activate _duckfeathers false))

(event EventBeginPlay
  (bind _trackbpref (Variables|Default|GetTrackBPRef))
  (|CallParentFunction)
  (Utilities|FlowControl|Delay 0.3)
  (Utilities|FlowControl|Sequence
    (:then_0
      (if (Variables|Default|GetbActiveDuck)
        (Utilities|IsValid _trackbpref
          (:Is%20Valid
            (CallFunction|MoveDuck)
            (Variables|Default|SetTrack_BPRef _trackbpref))
          (:Is%20Not%20Valid
            (Actor|DestroyActor)))))))

(event Collision|EventActorBeginOverlap
  (params (OtherActor :type Actor%20Object%20Reference))
  (|CallParentFunction OtherActor) ; This node is disabled and will not be called.\nDrag off pins to build functionality.
)

(event EventTick
  (params (DeltaSeconds :type Float%20%28single-precision%29))
  (|CallParentFunction DeltaSeconds) ; This node is disabled and will not be called.\nDrag off pins to build functionality.
)

(fn ConstructionScript
  (|CallParentFunction))

(fn BirdHIt
  (bind _returnvalue (Math|Random|RandomFloatinRange -3e+01 3e+01))
  (|CallParentFunction)
  (Components|Activation|Deactivate (Variables|Default|GetRipple))
  (Variables|Default|SetbHit true)
  (Transformation|SetRelativeRotation (Variables|Default|GetSK_BIrd) (Math|Rotator|MakeRotator _returnvalue _returnvalue (Math|Random|RandomFloatinRange -1.3e+02 -5e+01)) false false)
  (CallFunction|ReleaseFeathers))