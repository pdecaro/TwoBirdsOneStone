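; Hummingbird target, a child of a bird base class, that darts across the scene and counts as missed if it completes its flight.
; After starting a 2D buzz, it eases through five spawner targets in FromLeft-dependent order, using random hover pauses and positional jitter except at the middle one.
; At the exit point it notifies the player and destroys itself.
; A hit plays an animation, randomizes roll, fades the buzz and releases feathers.
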(event Custom|StopSound
  (Audio|Components|Audio|FadeOut (Variables|Default|GetHummingSound) 0.2 0.0 "Linear" :!class /Script/Engine.AudioComponent))

(event Custom|ReleaseFeathers
  (bind _hummingbirdfeathers (Variables|Default|GetHummingbirdFeathers))
  (Transformation|DetachFromComponent _hummingbirdfeathers "KeepWorld" "KeepWorld" "KeepRelative" true)
  (Components|Activation|Activate _hummingbirdfeathers false))

(event EventBeginPlay
  (bind _returnvalue (Math|Random|RandomFloatinRange -1e+02 1e+02))
  (bind _returnvalue_2 (Math|Random|RandomFloatinRange -1e+02 1e+02))
  (bind _returnvalue_3 (Math|Random|RandomFloatinRange -1e+02 1e+02))
  (bind _returnvalue_4 (Math|Random|RandomFloatinRange -1e+02 1e+02))
  (bind _returnvalue_5 (Math|Random|RandomFloatinRange -1e+02 1e+02))
  (bind _returnvalue_6 (Math|Random|RandomFloatinRange -1e+02 1e+02))
  (bind _returnvalue_7 (Math|Random|RandomFloatinRange -1e+02 1e+02))
  (bind _returnvalue_8 (Math|Random|RandomFloatinRange -1e+02 1e+02))
  (bind _hummingbirdspawnerref (Variables|Default|GetHummingbirdSpawnerRef))
  (bind _hummingbirdspawnerref_2 (Variables|Default|GetHummingbirdSpawnerRef))
  (bind _hummingbirdspawnerref_3 (Variables|Default|GetHummingbirdSpawnerRef))
  (bind _hummingbirdspawnerref_4 (Variables|Default|GetHummingbirdSpawnerRef))
  (bind _hummingbirdspawnerref_5 (Variables|Default|GetHummingbirdSpawnerRef))
  (bind _hummingbirdspawnerref_6 (Variables|Default|GetHummingbirdSpawnerRef))
  (bind _hummingbirdspawnerref_7 (Variables|Default|GetHummingbirdSpawnerRef))
  (bind _hummingbirdspawnerref_8 (Variables|Default|GetHummingbirdSpawnerRef))
  (bind _hummingbirdspawnerref_9 (Variables|Default|GetHummingbirdSpawnerRef))
  (bind _hummingbirdspawnerref_10 (Variables|Default|GetHummingbirdSpawnerRef))
  (bind _target03 (Variables|/Game/Birds/Spawners/HummingBird_Spawner.HummingBird_Spawner_C|GetTarget03 _hummingbirdspawnerref_2))
  (bind _target05 (Variables|/Game/Birds/Spawners/HummingBird_Spawner.HummingBird_Spawner_C|GetTarget05 _hummingbirdspawnerref_5))
  (bind _target04 (Variables|/Game/Birds/Spawners/HummingBird_Spawner.HummingBird_Spawner_C|GetTarget04 _hummingbirdspawnerref_6))
  (bind _target03_2 (Variables|/Game/Birds/Spawners/HummingBird_Spawner.HummingBird_Spawner_C|GetTarget03 _hummingbirdspawnerref_7))
  (bind _target02 (Variables|/Game/Birds/Spawners/HummingBird_Spawner.HummingBird_Spawner_C|GetTarget02 _hummingbirdspawnerref_8))
  (bind _target01 (Variables|/Game/Birds/Spawners/HummingBird_Spawner.HummingBird_Spawner_C|GetTarget01 _hummingbirdspawnerref_9))
  (bind _target01_2 (Variables|/Game/Birds/Spawners/HummingBird_Spawner.HummingBird_Spawner_C|GetTarget01 _hummingbirdspawnerref_10))
  (bind _target02_2 (Variables|/Game/Birds/Spawners/HummingBird_Spawner.HummingBird_Spawner_C|GetTarget02 _hummingbirdspawnerref))
  (bind _target04_2 (Variables|/Game/Birds/Spawners/HummingBird_Spawner.HummingBird_Spawner_C|GetTarget04 _hummingbirdspawnerref_3))
  (bind _target05_2 (Variables|/Game/Birds/Spawners/HummingBird_Spawner.HummingBird_Spawner_C|GetTarget05 _hummingbirdspawnerref_4))
  (bind _returnvalue_9 (Transformation|GetWorldTransform _target01_2))
  (bind _returnvalue_10 (Transformation|GetWorldTransform _target02_2))
  (bind _returnvalue_11 (Transformation|GetWorldTransform _target03))
  (bind _returnvalue_12 (Transformation|GetWorldTransform _target04_2))
  (bind _returnvalue_13 (Transformation|GetWorldTransform _target05_2))
  (bind _returnvalue_14 (Transformation|GetWorldTransform _target05))
  (bind _returnvalue_15 (Transformation|GetWorldTransform _target04))
  (bind _returnvalue_16 (Transformation|GetWorldTransform _target03_2))
  (bind _returnvalue_17 (Transformation|GetWorldTransform _target02))
  (bind _returnvalue_18 (Transformation|GetWorldTransform _target01))
  (|CallParentFunction)
  (Utilities|FlowControl|Delay 0.5)
  (Utilities|FlowControl|Sequence
    (:then_0
      (bind _returnvalue_19 (Audio|CreateSound2D "/Game/Audio/SoundEffects/Birds/HummingbirdBuzz01_Cue.HummingbirdBuzz01_Cue" 1.0 1.0 0.0 0))
      (bind _output_get (Variables|Default|SetHummingSound _returnvalue_19))
      (Audio|Components|Audio|Play _output_get 0.0))
    (:then_1
      (if (Variables|Default|GetFromLeft)
        (Components|MoveComponentTo (Variables|Default|GetRoot) (Math|Vector|MakeVector (+ (.x (.location _returnvalue_14)) _returnvalue_5) (+ (.y (.location _returnvalue_14)) _returnvalue_5) (+ (.z (.location _returnvalue_14)) _returnvalue_5)) "0, 0, 0" true true 0.5 false)
        (Utilities|FlowControl|Delay (Math|Random|RandomFloatinRange 1.25 1.75))
        (Components|MoveComponentTo (Variables|Default|GetRoot) (Math|Vector|MakeVector (+ (.x (.location _returnvalue_15)) _returnvalue_6) (+ (.y (.location _returnvalue_15)) _returnvalue_6) (+ (.z (.location _returnvalue_15)) _returnvalue_6)) "0, 0, 0" true true 0.5 false)
        (Utilities|FlowControl|Delay (Math|Random|RandomFloatinRange 1.25 1.75))
        (Components|MoveComponentTo (Variables|Default|GetRoot) (Math|Vector|MakeVector (+ (.x (.location _returnvalue_16)) 5e+01) (.y (.location _returnvalue_16)) (.z (.location _returnvalue_16))) "0, 0, 0" true true 0.5 false)
        (Utilities|FlowControl|Delay (Math|Random|RandomFloatinRange 1.25 1.75))
        (Components|MoveComponentTo (Variables|Default|GetRoot) (Math|Vector|MakeVector (+ (.x (.location _returnvalue_17)) _returnvalue_7) (+ (.y (.location _returnvalue_17)) _returnvalue_7) (+ (.z (.location _returnvalue_17)) _returnvalue_7)) "0, 0, 0" true true 0.5 false)
        (Utilities|FlowControl|Delay (Math|Random|RandomFloatinRange 1.25 1.75))
        (Components|MoveComponentTo (Variables|Default|GetRoot) (Math|Vector|MakeVector (+ (.x (.location _returnvalue_18)) _returnvalue_8) (+ (.y (.location _returnvalue_18)) _returnvalue_8) (+ (.z (.location _returnvalue_18)) _returnvalue_8)) "0, 0, 0" true true 0.5 false)
        (Utilities|FlowControl|Delay (Math|Random|RandomFloatinRange 3.0 3.5))
        (Components|MoveComponentTo (Variables|Default|GetRoot) (Transformation|GetWorldLocation (Variables|/Game/Birds/Spawners/HummingBird_Spawner.HummingBird_Spawner_C|GetSpawnLeftEnd (Variables|Default|GetHummingbirdSpawnerRef))) "0, 0, 0" true true 0.5 false)
        (else
          (Components|MoveComponentTo (Variables|Default|GetRoot) (Math|Vector|MakeVector (+ (.x (.location _returnvalue_9)) _returnvalue) (+ (.y (.location _returnvalue_9)) _returnvalue) (+ (.z (.location _returnvalue_9)) _returnvalue)) "0, 0, 0" true true 0.5 false)
          (Utilities|FlowControl|Delay (Math|Random|RandomFloatinRange 1.25 1.75))
          (Components|MoveComponentTo (Variables|Default|GetRoot) (Math|Vector|MakeVector (+ (.x (.location _returnvalue_10)) _returnvalue_2) (+ (.y (.location _returnvalue_10)) _returnvalue_2) (+ (.z (.location _returnvalue_10)) _returnvalue_2)) "0, 0, 0" true true 0.5 false)
          (Utilities|FlowControl|Delay (Math|Random|RandomFloatinRange 1.25 1.75))
          (Components|MoveComponentTo (Variables|Default|GetRoot) (Math|Vector|MakeVector (+ (.x (.location _returnvalue_11)) -5e+01) (.y (.location _returnvalue_11)) (.z (.location _returnvalue_11))) "0, 0, 0" true true 0.5 false)
          (Utilities|FlowControl|Delay (Math|Random|RandomFloatinRange 1.25 1.75))
          (Components|MoveComponentTo (Variables|Default|GetRoot) (Math|Vector|MakeVector (+ (.x (.location _returnvalue_12)) _returnvalue_3) (+ (.y (.location _returnvalue_12)) _returnvalue_3) (+ (.z (.location _returnvalue_12)) _returnvalue_3)) "0, 0, 0" true true 0.5 false)
          (Utilities|FlowControl|Delay (Math|Random|RandomFloatinRange 1.25 1.75))
          (Components|MoveComponentTo (Variables|Default|GetRoot) (Math|Vector|MakeVector (+ (.x (.location _returnvalue_13)) _returnvalue_4) (+ (.y (.location _returnvalue_13)) _returnvalue_4) (+ (.z (.location _returnvalue_13)) _returnvalue_4)) "0, 0, 0" true true 0.5 false)
          (Utilities|FlowControl|Delay (Math|Random|RandomFloatinRange 3.0 3.5))
          (Components|MoveComponentTo (Variables|Default|GetRoot) (Transformation|GetWorldLocation (Variables|/Game/Birds/Spawners/HummingBird_Spawner.HummingBird_Spawner_C|GetSpawnRightEnd (Variables|Default|GetHummingbirdSpawnerRef))) "0, 0, 0" true true 0.5 false)))
      (Default|MissedBird (Variables|Default|GetPlayerBPRef))
      (CallFunction|StopSound)
      (Utilities|FlowControl|Delay 0.21)
      (CallFunction|BirdDestroyed)
      (Actor|DestroyActor))))

(event Collision|EventActorBeginOverlap
  (params (OtherActor :type Actor%20Object%20Reference))
  (|CallParentFunction OtherActor) ; This node is disabled and will not be called.\nDrag off pins to build functionality.
)

(event EventTick
  (params (DeltaSeconds :type Float%20%28single-precision%29)))

(fn ConstructionScript
  (|CallParentFunction))

(fn BirdHIt
  (bind _sk_bird (Variables|Default|GetSK_BIrd))
  (bind _relativerotation (Variables|/Script/Engine.SceneComponent|GetRelativeRotation _sk_bird))
  (|CallParentFunction)
  (Components|Animation|PlayAnimation (Variables|Default|GetSK_BIrd) "/Game/Models/Birds/Hummingbird/Animations/Hummingbird_Hit_anim.Hummingbird_Hit_anim" true)
  (Transformation|SetRelativeRotation _sk_bird (Math|Rotator|MakeRotator (Math|Random|RandomFloatinRange 1.0 1.8e+02) (.pitch _relativerotation) (.yaw _relativerotation)) false false)
  (CallFunction|StopSound)
  (CallFunction|ReleaseFeathers))

(fn BirdDestroyed
  (|CallParentFunction)
  (CallFunction|StopSound))