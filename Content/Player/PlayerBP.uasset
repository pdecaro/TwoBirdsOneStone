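; Player Blueprint for a slingshot bird-shooting game, handling aiming, firing, pausing, saving and shot/hit/miss counts.
; Axis inputs pan and rotate the slingshot within limits, with optional Y inversion.
; Holding pull-back runs a looping timer that builds Power, driving camera zoom and stretch volume; release spawns a stone with power-scaled velocity.
; It routes menu input to pause and confirmation widgets, and syncs high scores and inversion between GameInstance and SaveGame.
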(event Custom|ResetSlingshot
  ;[1 1 1] Slingshot Control
  ;;[1 1 1] Aiming
  (Utilities|FlowControl|Sequence
    (:then_0
      (Utilities|FlowControl|Sequence
        (:then_0
          (Utilities|FlowControl|DoOnce false :!label _label
            (:Completed
              (bind _alpha (Timeline|SmoothReturn PlayFromStart)
                (:Update
                  (Variables|/Script/Engine.SpringArmComponent|SetTargetArmLength (Variables|Default|GetAimCameraBoom) (Math|Float|Lerp (Variables|Control|GetCurrentZoom) (Variables|Control|GetDefaultArmLength) _alpha))
                  (Utilities|FlowControl|Delay (Variables|Control|GetTimeUntilNextShot))
                  (Variables|Control|SetbCanAim true)
                  (Variables|Control|SetbCanShoot true)
                  (Variables|Aiming|SetbAiming true)
                  (Rendering|SetVisibility (Variables|Default|GetSM_Stone_01) true false))))))
        (:then_1
          (Utilities|FlowControl|Delay 0.4)
          (goto _label Reset))))))

(event Custom|UseAimCamera
  ;[1 1 1] Camera
  (Game|Player|SetViewTargetwithBlend (Game|GetPlayerController 0) self 0.3 "VTBlend_Linear" 1.0 true))

(event Custom|EnablePress
  ;[1 1 1] Player Controls
  (Variables|Control|SetbDisablePress true))

(event Custom|AddPower
  ;[1 1 1] Slingshot Control
  ;;[1 1 1] Set Power
  ;;;[1 1 1] Add Power
  (bind _output_get (Variables|Control|SetPower (Math|Float|Clamp(Float) (+ (Variables|Control|GetPower) 3.0) 1e+01 1e+02)))
  (bind _output_get_2 (Variables|/Script/Engine.SpringArmComponent|SetTargetArmLength (Variables|Default|GetAimCameraBoom) (Math|Float|Lerp (Variables|Control|GetDefaultArmLength) (Variables|Control|GetZoomMax) (/ _output_get 1e+02))))
  (Variables|Control|SetCurrentZoom _output_get_2))

(event Custom|StoneFired
  ;[1 1 1] Slingshot Control
  ;;[1 1 1] Aiming
  (Variables|Aiming|SetbAiming false)
  (if (>= (Variables|Control|GetPower) 1.0)
    (CallFunction|ShootSoundFX)
    (Utilities|FlowControl|Delay 0.005)
    (CallFunction|FireStone)
    (CallFunction|ResetSlingshot)
    (Rendering|SetVisibility (Variables|Default|GetSM_Stone_01) false false)))

(event Custom|PlayWaveJingle
  ;[1 1 1] Wave Jingle
  (Audio|PlaySound2D "/Game/Audio/SoundEffects/Jingles/WaveJingles01_Cue.WaveJingles01_Cue" 1.0 1.0 0.0 0 0))

(event Custom|PausePausing
  (params (bCanPauseGame :type Boolean))
  ;[1 1 1] Paused and Saved
  (Variables|Default|SetbCanPauseGame bCanPauseGame))

(event Custom|TempPausePause
  ;[1 1 1] Paused and Saved
  (Variables|Default|SetbCanPauseGame false)
  (Utilities|FlowControl|Delay 3.5)
  (Variables|Default|SetbCanPauseGame true))

(event Custom|AreYouSureUI
  ;[1 1 1] Paused and Saved
  (bind _returnvalue (UserInterface|CreateWidget "/Game/UI/AreYouSureUI.AreYouSureUI_C"))
  (bind _output_get (Variables|Default|SetAreYouSureUIRef _returnvalue))
  (UserInterface|Viewport|AddtoViewport _output_get 0))

(event Custom|ExitPause
  ;[1 1 1] Paused and Saved
  (Utilities|IsValid (Variables|Default|GetPauseMenuWidgetRef)
    (:Is%20Valid
      (Widget|RemovefromParent (Variables|Default|GetPauseMenuWidgetRef))
      (Variables|Default|SetPauseMenuWidgetRef 0)
      (bind _returnvalue (UserInterface|CreateWidget "/Game/UI/PauseMenu.PauseMenu_C"))
      (bind _output_get (Variables|Default|SetPauseMenuWidgetRef _returnvalue))
      (UserInterface|Viewport|AddtoViewport _output_get 0))))

(event Custom|SaveGame
  (bind _gameinstref (Variables|Refs|GetGameINSTRef))
  ;[1 1 1] Paused and Saved
  ;;[1 1 1] Save Game
  (bind _returnvalue (SaveGame|DoesSaveGameExist (Variables|Default|GetSaveGame01)))
  (if _returnvalue
    (bind _returnvalue_2 (SaveGame|LoadGamefromSlot (Variables|Default|GetSaveGame01)))
    (bind _output_get (Variables|Default|SetSaverSubclass _returnvalue_2))
    (bind _assave_game_01 (Utilities|Casting|CastToSaveGame01 _output_get))
    (Variables|/Game/Player/SaveGame01.SaveGame01_C|SetGameAHighScore _assave_game_01 (Variables|/Game/Player/TBOS_GameInstance.TBOS_GameInstance_C|GetGameAHighScore _gameinstref))
    (Variables|/Game/Player/SaveGame01.SaveGame01_C|SetGameBHighScore _assave_game_01 (Variables|/Game/Player/TBOS_GameInstance.TBOS_GameInstance_C|GetGameBHighScore _gameinstref))
    (Variables|/Game/Player/SaveGame01.SaveGame01_C|SetbInvertControls _assave_game_01 (Variables|/Game/Player/TBOS_GameInstance.TBOS_GameInstance_C|GetbInvertControls _gameinstref))
    (else
      (bind _returnvalue_3 (SaveGame|CreateSaveGameObject "/Game/Player/SaveGame01.SaveGame01_C"))
      (bind _output_get_2 (Variables|Default|SetSaverSubclass _returnvalue_3))
      (bind _assave_game_01_2 (Utilities|Casting|CastToSaveGame01 _output_get_2))
      (Variables|/Game/Player/SaveGame01.SaveGame01_C|SetGameAHighScore _assave_game_01_2 (Variables|/Game/Player/TBOS_GameInstance.TBOS_GameInstance_C|GetGameAHighScore _gameinstref))
      (Variables|/Game/Player/SaveGame01.SaveGame01_C|SetGameBHighScore _assave_game_01_2 (Variables|/Game/Player/TBOS_GameInstance.TBOS_GameInstance_C|GetGameBHighScore _gameinstref))
      (Variables|/Game/Player/SaveGame01.SaveGame01_C|SetbInvertControls _assave_game_01_2 (Variables|/Game/Player/TBOS_GameInstance.TBOS_GameInstance_C|GetbInvertControls _gameinstref))))
  (SaveGame|SaveGametoSlot (Variables|Default|GetSaverSubclass) (Variables|Default|GetSaveGame01)))

(event Custom|LoadGame
  (bind _gameinstref (Variables|Refs|GetGameINSTRef))
  ;[1 1 1] Paused and Saved
  (bind _returnvalue (SaveGame|DoesSaveGameExist (Variables|Default|GetSaveGame01)))
  (if _returnvalue
    (bind _returnvalue_2 (SaveGame|LoadGamefromSlot (Variables|Default|GetSaveGame01)))
    (bind _output_get (Variables|Default|SetSaverSubclass _returnvalue_2))
    (bind _assave_game_01 (Utilities|Casting|CastToSaveGame01 _output_get))
    (Utilities|FlowControl|Sequence
      (:then_0
        (Variables|/Game/Player/TBOS_GameInstance.TBOS_GameInstance_C|SetGameAHighScore _gameinstref (Variables|/Game/Player/SaveGame01.SaveGame01_C|GetGameAHighScore _assave_game_01)))
      (:then_1
        (Variables|/Game/Player/TBOS_GameInstance.TBOS_GameInstance_C|SetGameBHighScore _gameinstref (Variables|/Game/Player/SaveGame01.SaveGame01_C|GetGameBHighScore _assave_game_01)))
      (:then_2
        (bind _output_get_2 (Variables|/Game/Player/TBOS_GameInstance.TBOS_GameInstance_C|SetbInvertControls _gameinstref (Variables|/Game/Player/SaveGame01.SaveGame01_C|GetbInvertControls _assave_game_01)))
        (Variables|Default|SetbInvertY _output_get_2)))))

(event Custom|ResetSlingShotLocation
  (bind _slingshot02 (Variables|Default|GetSlingshot02))
  ;[1 1 1] Camera
  (bind _alpha (Timeline|Timeline_0 PlayFromStart)
    (:Update
      (Transformation|SetRelativeRotation _slingshot02 (Math|Rotator|Lerp(Rotator) (Variables|/Script/Engine.SceneComponent|GetRelativeRotation _slingshot02) "0,90.000000, 0" _alpha true) false false))))

(event Custom|FireStone
  (bind _stretchstartsound (Variables|Default|GetStretchStartSound))
  ;[1 1 1] Fire Stone
  (Utilities|FlowControl|Sequence
    (:then_0
      (Utilities|FlowControl|DoOnce false :!label _label
        (:Completed
          (CallFunction|ShotsFired)
          (bind _returnvalue (Game|SpawnActorfromClass "/Game/Projectile/StoneProjectile_BP.StoneProjectile_BP_C" (Transformation|GetWorldTransform (Variables|Default|GetProjectilePivot)) "Undefined" 0 1e+03 0))
          (bind _output_get (Variables|Refs|SetStoneBPRef _returnvalue))
          (Variables|/Script/Engine.MovementComponent|SetVelocity (Variables|/Game/Projectile/StoneProjectile_BP.StoneProjectile_BP_C|GetProjectileMovement _returnvalue) (* (Math|Vector|GetForwardVector (Variables|/Game/Projectile/StoneProjectile_BP.StoneProjectile_BP_C|GetStone _output_get)) (Math|Float|Clamp(Float) (* (Variables|/Script/Engine.ProjectileMovementComponent|GetInitialSpeed (Variables|/Game/Projectile/StoneProjectile_BP.StoneProjectile_BP_C|GetProjectileMovement _returnvalue)) (Math|Float|Clamp(Float) (/ (Variables|Control|GetPower) 1e+02) 0.2)) 8e+02 5e+03)))
          (Variables|Aiming|SetbLoaded false))))
    (:then_1
      (Utilities|FlowControl|Delay 0.2)
      (goto _label Reset))
    (:then_2
      ;[1 1 1] Slingshot Control
      ;;[1 1 1] Set Power
      (CallFunction|StopStretchSound)
      (Utilities|IsValid _stretchstartsound
        (:Is%20Valid
          (Audio|Components|Audio|Stop _stretchstartsound)
          (Utilities|FlowControl|DoOnce false) ; enters at Reset
        )
        (:Is%20Not%20Valid
          (Utilities|FlowControl|DoOnce false) ; enters at Reset
        )))))

(event Custom|CancelSlingshot
  ;[1 1 1] Slingshot Control
  ;;[1 1 1] Aiming
  (CallFunction|StopStretchSound)
  (Variables|Control|SetbCanAim false)
  (Variables|Aiming|SetbLoaded false)
  (Variables|Aiming|SetbAiming false)
  (Variables|Control|SetPower 0.0)
  (Utilities|FlowControl|Delay 0.2)
  (CallFunction|ResetSlingShotLocation))

(event Custom|ShootSoundFX
  (bind _returnvalue (Math|Random|RandomFloatinRange 0.8 1.2))
  (bind _slingshot02 (Variables|Default|GetSlingshot02))
  (bind _returnvalue_2 (Transformation|GetWorldLocation _slingshot02))
  ;[1 1 1] Fire Stone
  (if (<= (Variables|Control|GetPower) 5e+01)
    (Audio|PlaySoundatLocation "/Game/Audio/SoundEffects/SlingShot/ShootStone04_Cue.ShootStone04_Cue" _returnvalue_2 "0, 0, 0" 1.0 _returnvalue 0.0 0 0 0)
    (else
      (Audio|PlaySoundatLocation "/Game/Audio/SoundEffects/SlingShot/ShootStone03_Cue.ShootStone03_Cue" _returnvalue_2 "0, 0, 0" 1.0 _returnvalue 0.0 0 0 0))))

(event Custom|StopStretchSound
  (bind _stretchstartsound (Variables|Default|GetStretchStartSound))
  ;[1 1 1] Slingshot Control
  ;;[1 1 1] Set Power
  (Audio|Components|Audio|Stop (Variables|Default|GetStretchLoop))
  (Utilities|IsValid _stretchstartsound
    (:Is%20Valid
      (Audio|Components|Audio|Stop _stretchstartsound)
      (Utilities|FlowControl|DoOnce false) ; enters at Reset
    )
    (:Is%20Not%20Valid
      (Utilities|FlowControl|DoOnce false) ; enters at Reset
    )))

(event Custom|StartGame
  ;[1 1 1] StartGame
  (Variables|Default|SetbStartGame true)
  (Utilities|FlowControl|Sequence
    (:then_0
      (Rendering|SetVisibility (Variables|Default|GetRoot) true true))
    (:then_1
      (CallFunction|UseAimCamera))
    (:then_2
      (Transformation|AttachComponentToComponent (Variables|Default|GetSM_Stone_01) (Variables|Default|GetStraps) "Stone" "SnapToTarget" "SnapToTarget" "KeepRelative" true))
    (:then_3
      (bind _returnvalue (Audio|CreateSound2D "/Game/Audio/SoundEffects/SlingShot/Stretching_Loop_Cue.Stretching_Loop_Cue" 1.0 1.0 0.0 0 false false))
      (Variables|Default|SetStretchLoop _returnvalue))))

(event Custom|ResetSlingshotAim
  ;[1 1 1] Slingshot Control
  ;;[1 1 1] Aiming
  (Utilities|FlowControl|Sequence
    (:then_0
      (Utilities|FlowControl|DoOnce false :!label _label
        (:Completed
          (bind _alpha (Timeline|SmoothReturn PlayFromStart)
            (:Update
              (Variables|/Script/Engine.SpringArmComponent|SetTargetArmLength (Variables|Default|GetAimCameraBoom) (Math|Float|Lerp (Variables|Control|GetCurrentZoom) (Variables|Control|GetDefaultArmLength) _alpha))
              (Utilities|FlowControl|Delay (Variables|Control|GetTimeUntilNextShot))
              (Variables|Control|SetbCanAim true)
              (Variables|Control|SetbCanShoot true)
              (Variables|Aiming|SetbAiming true)
              (Rendering|SetVisibility (Variables|Default|GetSM_Stone_01) true false))))))
    (:then_1
      (Utilities|FlowControl|Delay 0.4)
      (goto _label Reset))))

(event Custom|DisablePress
  ;[1 1 1] Player Controls
  (Variables|Control|SetbDisablePress true))

(event EventBeginPlay
  (bind _slingshot02 (Variables|Default|GetSlingshot02))
  (bind _relativelocation (Variables|/Script/Engine.SceneComponent|GetRelativeLocation _slingshot02))
  ;[1 1 1] Begin Play
  (Utilities|FlowControl|Sequence
    (:then_0
      (Input|DisableInput 0))
    (:then_1
      (|SetOurRefs))
    (:then_2
      (Rendering|SetVisibility (Variables|Default|GetRoot) false true))
    (:then_3
      (Transformation|SetRelativeLocation _slingshot02 (Math|Vector|MakeVector (.x _relativelocation) (.y _relativelocation) (+ (.z _relativelocation) 3.5e+02)) false false))))

(event EventTick
  (params (DeltaSeconds :type Float%20%28single-precision%29))
  ;[1 1 1] Event Tick
  (if (Variables|Aiming|GetbLoaded)
    (bind _output_get (Variables|Default|SetStretchVolume (/ (Variables|Control|GetPower) 1e+02)))
    (Audio|Components|Audio|AdjustVolume (Variables|Default|GetStretchLoop) 0.1 _output_get "Linear" :!class /Script/Engine.AudioComponent)))

(event Input|ActionEvents|InputActionPause
  (params (Key :type Key%20Structure :default "None"))
  ;[1 1 1] Paused and Saved
  (:Pressed
    (if (Variables|Default|GetbCanPauseGame)
      (if (Variables|Default|GetbGamePaused)
        (Game|SetGamePaused false)
        (Variables|Default|SetbGamePaused false)
        (Utilities|IsValid (Variables|Default|GetPauseMenuWidgetRef)
          (:Is%20Valid
            (Widget|RemovefromParent (Variables|Default|GetPauseMenuWidgetRef))
            (Variables|Default|SetPauseMenuWidgetRef 0)))
        (else
          (bind _returnvalue (Game|SetGamePaused true))
          (Variables|Default|SetbGamePaused _returnvalue)
          (bind _returnvalue_2 (UserInterface|CreateWidget "/Game/UI/PauseMenu.PauseMenu_C"))
          (bind _output_get (Variables|Default|SetPauseMenuWidgetRef _returnvalue_2))
          (UserInterface|Viewport|AddtoViewport _output_get 0)))
      (elif (Variables|Default|GetbGamePaused)
        (Game|SetGamePaused false)
        (Variables|Default|SetbGamePaused false)
        (Utilities|IsValid (Variables|Default|GetPauseMenuWidgetRef)
          (:Is%20Valid
            (Widget|RemovefromParent (Variables|Default|GetPauseMenuWidgetRef))
            (Variables|Default|SetPauseMenuWidgetRef 0)))))))

(event Input|ActionEvents|InputActionCancelAim
  (params (Key :type Key%20Structure :default "None"))
  ;[1 1 1] Slingshot Control
  ;;[1 1 1] Aiming
)

(event Input|ActionEvents|InputActionPullBackStart
  (params (Key :type Key%20Structure :default "None"))
  ;[1 1 1] Slingshot Control
  ;;[1 1 1] Set Power
  (:Pressed
    (Utilities|FlowControl|Sequence
      (:then_0
        (if (== (Variables|Control|GetPower) 0.0)
          (Utilities|FlowControl|DoOnce false :!label _label)
          (else
            (goto _label Reset))))
      (:then_1
        (Utilities|Time|SetTimerbyFunctionName 0 "AddPower" 0.01 true)
        (Variables|Aiming|SetbLoaded true)
        (bind _returnvalue (Audio|CreateSound2D "/Game/Audio/SoundEffects/SlingShot/Stretching_Start02_Cue.Stretching_Start02_Cue" 1.0 1.0 0.0 0))
        (bind _output_get (Variables|Default|SetStretchStartSound _returnvalue))
        (Audio|Components|Audio|Play _output_get 0.0))
      (:then_2
        (Utilities|FlowControl|DoOnce false
          (:Completed
            (Audio|Components|Audio|Play (Variables|Default|GetStretchLoop) 0.0))))))
  (:Released
    (if (Variables|Aiming|GetbAiming)
      (CallFunction|FireStone)
      (CallFunction|StoneFired)
      (Utilities|Time|ClearTimerbyFunctionName 0 "AddPower")
      (Variables|Control|SetPower 0.0)
      (CallFunction|StopStretchSound)
      (else
        (Variables|Aiming|SetbLoaded false)
        (Variables|Aiming|SetbAiming false)
        (Utilities|Time|ClearTimerbyFunctionName 0 "AddPower")
        (Variables|Control|SetPower 0.0)
        (CallFunction|ResetSlingshot)
        (CallFunction|StopStretchSound)))))

(event Input|ActionEvents|InputActionAcceptChoice
  (params (Key :type Key%20Structure :default "None"))
  (bind _pausemenuwidgetref (Variables|Default|GetPauseMenuWidgetRef))
  (bind _areyousureuiref (Variables|Default|GetAreYouSureUIRef))
  ;[1 1 1] Paused and Saved
  (:Pressed
    (if (Variables|Default|GetbAreYouSureMenuOpen)
      (Utilities|IsValid _areyousureuiref
        (:Is%20Valid
          (Default|AcceptChoice _areyousureuiref)))
      (else
        (Utilities|IsValid _pausemenuwidgetref
          (:Is%20Valid
            (Default|AcceptChoice _pausemenuwidgetref)))))))

(event Input|ActionEvents|InputActionCanPan
  (params (Key :type Key%20Structure :default "None"))
  ;[1 1 1] Slingshot Control
  ;;[1 1 1] Aiming
  (:Pressed
    (Variables|Control|SetbCanPan true))
  (:Released
    (Variables|Control|SetbCanPan false)))

(event Input|ActionEvents|InputActionSwitchUp
  (params (Key :type Key%20Structure :default "None"))
  (bind _pausemenuwidgetref (Variables|Default|GetPauseMenuWidgetRef))
  (bind _areyousureuiref (Variables|Default|GetAreYouSureUIRef))
  ;[1 1 1] Paused and Saved
  (:Pressed
    (if (Variables|Default|GetbAreYouSureMenuOpen)
      (Utilities|IsValid _areyousureuiref
        (:Is%20Valid
          (Default|Switch _areyousureuiref)))
      (else
        (Utilities|IsValid _pausemenuwidgetref
          (:Is%20Valid
            (Default|SwitchUp _pausemenuwidgetref)))))))

(event Input|ActionEvents|InputActionSwitchDown
  (params (Key :type Key%20Structure :default "None"))
  (bind _pausemenuwidgetref (Variables|Default|GetPauseMenuWidgetRef))
  (bind _areyousureuiref (Variables|Default|GetAreYouSureUIRef))
  ;[1 1 1] Paused and Saved
  (:Pressed
    (if (Variables|Default|GetbAreYouSureMenuOpen)
      (Utilities|IsValid _areyousureuiref
        (:Is%20Valid
          (Default|Switch _areyousureuiref)))
      (else
        (Utilities|IsValid _pausemenuwidgetref
          (:Is%20Valid
            (Default|SwitchDown _pausemenuwidgetref)))))))

(event Input|AxisEvents|InputAxisPanUp
  (params (AxisValue :type Float%20%28single-precision%29))
  ;[1 1 1] Slingshot Control
  ;;[1 1 1] Panning
  (|PanningUp AxisValue))

(event Input|AxisEvents|InputAxisPanRight
  (params (AxisValue :type Float%20%28single-precision%29))
  ;[1 1 1] Slingshot Control
  ;;[1 1 1] Panning
  (|PanningRight AxisValue))

(event Input|AxisEvents|InputAxisPreciseRotRight
  (params (AxisValue :type Float%20%28single-precision%29))
  (bind _amounttoturn (Variables|Control|GetAmountToTurn))
  (bind _slingshot02 (Variables|Default|GetSlingshot02))
  (bind _relativerotation (Variables|/Script/Engine.SceneComponent|GetRelativeRotation _slingshot02))
  ;[1 1 1] Slingshot Control
  ;;[1 1 1] Precision Aiming
  (Transformation|SetRelativeRotation _slingshot02 (Math|Rotator|MakeRotator (.roll _relativerotation) (.pitch _relativerotation) (Math|Float|Clamp(Float) (+ (.yaw _relativerotation) (/ AxisValue (/ (Variables|Control|GetConstantSpeed) (Variables|PlayerVariables|GetPrecisionAimingSpeed)))) (- 9e+01 _amounttoturn) (+ 9e+01 _amounttoturn))) false false))

(event Input|AxisEvents|InputAxisPreciseRotUp
  (params (AxisValue :type Float%20%28single-precision%29))
  (bind _amounttotilt (Variables|Control|GetAmountToTilt))
  (bind _slingshot02 (Variables|Default|GetSlingshot02))
  (bind _amounttotilt_2 (Variables|Control|GetAmountToTilt))
  (bind _slingshot02_2 (Variables|Default|GetSlingshot02))
  (bind _relativerotation (Variables|/Script/Engine.SceneComponent|GetRelativeRotation _slingshot02))
  (bind _relativerotation_2 (Variables|/Script/Engine.SceneComponent|GetRelativeRotation _slingshot02_2))
  ;[1 1 1] Slingshot Control
  ;;[1 1 1] Precision Aiming
  (if (not (Variables|Default|GetbInvertY))
    (Transformation|SetRelativeRotation _slingshot02 (Math|Rotator|MakeRotator (Math|Float|Clamp(Float) (+ (.roll _relativerotation) (/ AxisValue (/ (Variables|Control|GetConstantSpeed) (Variables|PlayerVariables|GetPrecisionAimingSpeed)))) (* _amounttotilt_2 -1.0) _amounttotilt_2) (.pitch _relativerotation) (.yaw _relativerotation)) false false)
    (else
      (Transformation|SetRelativeRotation _slingshot02_2 (Math|Rotator|MakeRotator (Math|Float|Clamp(Float) (+ (.roll _relativerotation_2) (/ (* AxisValue -1.0) (/ (Variables|Control|GetConstantSpeed) (Variables|PlayerVariables|GetPrecisionAimingSpeed)))) (* _amounttotilt -1.0) _amounttotilt) (.pitch _relativerotation_2) (.yaw _relativerotation_2)) false false))))

(fn ConstructionScript)

(fn MissedBird
  (bind _birdsleftuiref (Variables|Default|GetBirdsLeftUIRef))
  (bind _result (Math|Integer|IncrementInt (Variables|Stats|GetBirdsMissed))
    (:%20%20
      (Variables|Stats|SetBirdsMissed _result)
      (if (not (Variables|Default|GetbGameModeA))
        (bind _output_get (Variables|Default|SetBirdsLeftGameB (Math|Integer|Clamp(Integer) (- (Variables|Default|GetBirdsLeftGameB) 1) 0 1000)))
        (Utilities|IsValid _birdsleftuiref
          (:Is%20Valid
            (Default|UpdateBirdsLeft _birdsleftuiref)
            (if (<= _output_get 0)
              (Default|CallGameBGameOver))))))))

(fn HitBird
  (bind _result (Math|Integer|IncrementInt (Variables|Stats|GetBirdsHit))
    (:%20%20
      (Variables|Stats|SetBirdsHit _result))))

(fn ShotsFired
  (bind _result (Math|Integer|IncrementInt (Variables|Stats|GetShots))
    (:%20%20
      (Variables|Stats|SetShots _result))))