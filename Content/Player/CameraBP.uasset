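; Standalone player camera Blueprint with a spring arm boom, which becomes the view target on BeginPlay.
; SetCameraArmLength zooms the arm between its default length and Zoom03 from a 0–100 Power input.
; ResetCamera blends the view back to this camera while the SmoothReturn timeline eases the arm to its default length.
; Player-tracking movement and tilt logic is present but disconnected, and Tick is empty.
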(event Custom|ResetCamera
  ;[1 1 1] Use Camera BP
  (Game|Player|SetViewTargetwithBlend (Game|GetPlayerController 0) self 0.2 "VTBlend_Linear" 1.0 true)
  (bind _alpha (Timeline|SmoothReturn PlayFromStart)
    (:Update
      (bind _output_get (Variables|/Script/Engine.SpringArmComponent|SetTargetArmLength (Variables|Default|GetCameraBoom) (Math|Float|Lerp (Variables|Default|GetCurrentCameraArmLength) (Variables|Default|GetDefaultCameraArmLength) _alpha)))
      (Variables|Default|SetCurrentCameraArmLength _output_get))))

(event Custom|SetCameraArmLength
  (params (Power :type Float%20%28single-precision%29))
  (bind _output_get (Variables|/Script/Engine.SpringArmComponent|SetTargetArmLength (Variables|Default|GetCameraBoom) (Math|Float|Clamp(Float) (Math|Float|Lerp (Variables|Default|GetDefaultCameraArmLength) (Variables|Default|GetZoom03) (/ Power 1e+02)) (Variables|Default|GetZoom03) (Variables|Default|GetDefaultCameraArmLength))))
  (Variables|Default|SetCurrentCameraArmLength _output_get))

(event EventBeginPlay
  ;[1 1 1] Begin Play
  (Utilities|FlowControl|Sequence
    (:then_0
      (Game|Player|SetViewTargetwithBlend (Game|GetPlayerController 0) self 0.0 "VTBlend_Linear" 0.0 false))))

(event EventTick
  (params (DeltaSeconds :type Float%20%28single-precision%29))
  ;[1 1 1] Event Tick
)

(fn ConstructionScript)