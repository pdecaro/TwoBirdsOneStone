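; Stone projectile that the player scores with by hitting birds, showing a bonus widget and raising the score multiplier on repeat hits.
; It enables physics on spawn, then after a fixed lifetime adds score times multiplier to PlayerBP's round score, updates the UI and destroys itself.
; Hits play throttled, pitch-randomized grass or stone sounds by physical surface.
; A one-shot splash fires effects, stops physics and hides the stone.
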(event OnComponentHit(Stone)
  (params (HitComponent :type Primitive%20Component%20Object%20Reference) (OtherActor :type Actor%20Object%20Reference) (OtherComp :type Primitive%20Component%20Object%20Reference) (NormalImpulse :type Vector :default "0, 0, 0") (Hit :type Hit%20Result%20Structure%20%28by%20ref%29))
  (bind (_bblockinghit _binitialoverlap _time _distance _location _impactpoint _normal _impactnormal _physmat) (Collision|BreakHitResult Hit))
  ;[1 1 1] Sounds
  (switch Utilities|FlowControl|Switch|SwitchonSurfaceTypes (Utilities|Select :Index (Variables|/Script/PhysicsCore.PhysicalMaterial|GetSurfaceType _physmat) :SurfaceType_Default "NewEnumerator2" :SurfaceType1 "NewEnumerator1" :SurfaceType2 "NewEnumerator2")
    (:NewEnumerator1
      (CallFunction|GrassSound _location))
    (:NewEnumerator2
      (CallFunction|StoneSound _location))))

(event Custom|Splash
  (bind _stone (Variables|Default|GetStone))
  (bind _relativelocation (Variables|/Script/Engine.SceneComponent|GetRelativeLocation _stone))
  ;[1 1 1] Splash
  (Utilities|FlowControl|DoOnce false
    (:Completed
      (Audio|PlaySoundatLocation "/Game/Audio/SoundEffects/Water/Stone_Splash_01_Cue.Stone_Splash_01_Cue" (Transformation|GetWorldLocation (Variables|Default|GetStone)) "0, 0, 0" 1.0 (Math|Random|RandomFloatinRange 0.8 1.2) 0.0 0 0 0)
      (Transformation|DetachFromComponent (Variables|Default|GetNS_Stylized_Splash_12) "KeepWorld" "KeepRelative" "KeepRelative" true)
      (Components|Activation|Activate (Variables|Default|GetSplashHit) true)
      (Physics|SetSimulatePhysics (Variables|Default|GetStone) false)
      (Utilities|FlowControl|Sequence
        (:then_0
          (Utilities|FlowControl|Delay 0.3)
          (Collision|SetCollisionEnabled (Variables|Default|GetStone) "NoCollision"))
        (:then_1
          (Components|MoveComponentTo _stone (Math|Vector|MakeVector (.x _relativelocation) (.y _relativelocation) (- (.z _relativelocation) 4e+01)) (Variables|/Script/Engine.SceneComponent|GetRelativeRotation _stone) false false 0.2 false)
          (Variables|Default|SetbDeadStone true)
          (Rendering|SetVisibility (Variables|Default|GetStone) false false))))))

(event Custom|GrassSound
  (params (Location :type Vector))
  ;[1 1 1] Sounds
  (if (Variables|Default|GetbCanPlaySound)
    (if (> (.X (Math|Vector|BreakVector (Transformation|GetComponentVelocity (Variables|Default|GetStone)))) 5e+02)
      (Variables|Default|SetbCanPlaySound false)
      (Audio|PlaySoundatLocation "/Game/Audio/SoundEffects/Impacts/HitGround_Grass_01_Cue.HitGround_Grass_01_Cue" Location "0, 0, 0" 1.0 (Math|Random|RandomFloatinRange 0.8 1.2) 0.0 0 0 0)
      (Utilities|FlowControl|Delay 0.2)
      (Variables|Default|SetbCanPlaySound true)
      (else
        (Variables|Default|SetbCanPlaySound false)
        (Audio|PlaySoundatLocation "/Game/Audio/SoundEffects/Impacts/HitGround_Grass_01_Cue.HitGround_Grass_01_Cue" (Transformation|GetWorldLocation (Variables|Default|GetStone)) "0, 0, 0" 0.3 (Math|Random|RandomFloatinRange 0.8 1.2) 0.0 0 0 0)
        (Utilities|FlowControl|Delay 0.2)
        (Variables|Default|SetbCanPlaySound true)))))

(event Custom|StoneSound
  (params (Location :type Vector))
  ;[1 1 1] Sounds
  (if (Variables|Default|GetbCanPlaySound)
    (if (> (.X (Math|Vector|BreakVector (Transformation|GetComponentVelocity (Variables|Default|GetStone)))) 5e+02)
      (Variables|Default|SetbCanPlaySound false)
      (Audio|PlaySoundatLocation "/Game/Audio/SoundEffects/Impacts/HitGround_Stone_01_Cue.HitGround_Stone_01_Cue" Location "0, 0, 0" 1.0 (Math|Random|RandomFloatinRange 0.8 1.2) 0.0 0 0 0)
      (Utilities|FlowControl|Delay 0.2)
      (Variables|Default|SetbCanPlaySound true)
      (else
        (Variables|Default|SetbCanPlaySound false)
        (Audio|PlaySoundatLocation "/Game/Audio/SoundEffects/Impacts/HitGround_Stone_01_Cue.HitGround_Stone_01_Cue" (Transformation|GetWorldLocation (Variables|Default|GetStone)) "0, 0, 0" 0.3 (Math|Random|RandomFloatinRange 0.8 1.2) 0.0 0 0 0)
        (Utilities|FlowControl|Delay 0.2)
        (Variables|Default|SetbCanPlaySound true)))))

(event Custom|FinishStone
  (bind _playerbpref (Variables|Default|GetPlayerBPRef))
  (bind _playerbpref_2 (Variables|Default|GetPlayerBPRef))
  (bind _playerbpref_3 (Variables|Default|GetPlayerBPRef))
  (bind _birdsleftuiref (Variables|/Game/Player/PlayerBP.PlayerBP_C|GetBirdsLeftUIRef _playerbpref_3))
  (bind _gamescoreuiref (Variables|/Game/Player/PlayerBP.PlayerBP_C|GetGameScoreUIRef _playerbpref))
  ;[1 1 1] Finish Stone, Add Score
  (Variables|Default|SetbDeadStone true)
  (bind _output_get (Variables|Default|SetFinalScoreForStone (* (Variables|Default|GetCurrentScore) (Variables|Default|GetCurrentMultiplier))))
  (bind _output_get_2 (Variables|/Game/Player/PlayerBP.PlayerBP_C|SetRoundScore _playerbpref_2 (+ _output_get (Variables|/Game/Player/PlayerBP.PlayerBP_C|GetRoundScore _playerbpref_2))))
  (Utilities|FlowControl|Sequence
    (:then_0
      (Utilities|IsValid _birdsleftuiref
        (:Is%20Valid
          (Default|UpdateScore _birdsleftuiref _output_get_2))))
    (:then_1
      (Utilities|IsValid _gamescoreuiref
        (:Is%20Valid
          (Default|UpdateScore _gamescoreuiref _output_get_2))))))

(event Custom|DisplayBonusText
  ;[1 1 1] Display Bonus Text
  (if (Variables|Default|GetbWidgetDisplayed)
    (Utilities|IsValid (Variables|Default|GetCurrentWidgetRef)
      (:Is%20Valid
        (Widget|RemovefromParent (Variables|Default|GetCurrentWidgetRef))
        (Variables|Default|SetCurrentWidgetRef 0)
        (bind _returnvalue (UserInterface|CreateWidget "/Game/UI/Birds1Stone_UI.Birds1Stone_UI_C" 0 0))
        (bind _output_get (Variables|Default|SetCurrentWidgetRef _returnvalue))
        (Variables|/Game/UI/Birds1Stone_UI.Birds1Stone_UI_C|SetStoneBPRef _output_get self)
        (UserInterface|Viewport|AddtoViewport _output_get 0)
        (Utilities|FlowControl|RetriggerableDelay 0.8)
        (Utilities|IsValid (Variables|Default|GetCurrentWidgetRef)
          (:Is%20Valid
            (Widget|RemovefromParent (Variables|Default|GetCurrentWidgetRef))))))
    (else
      (Variables|Default|SetbWidgetDisplayed true)
      (bind _returnvalue_2 (UserInterface|CreateWidget "/Game/UI/Birds1Stone_UI.Birds1Stone_UI_C" 0 0))
      (bind _output_get_2 (Variables|Default|SetCurrentWidgetRef _returnvalue_2))
      (Variables|/Game/UI/Birds1Stone_UI.Birds1Stone_UI_C|SetStoneBPRef _output_get_2 self)
      (UserInterface|Viewport|AddtoViewport _output_get_2 0)
      (Utilities|FlowControl|Delay 0.8)
      (Utilities|IsValid (Variables|Default|GetCurrentWidgetRef)
        (:Is%20Valid
          (Widget|RemovefromParent (Variables|Default|GetCurrentWidgetRef)))))))

(event EventBeginPlay
  ;[1 1 1] Begin Play
  (Utilities|FlowControl|Sequence
    (:then_0
      (bind _asplayer_bp (Utilities|Casting|CastToPlayerBP (Game|Player|GetPlayerPawn 0)))
      (Variables|Default|SetPlayerBPRef _asplayer_bp))
    (:then_1
      (Utilities|FlowControl|Delay 0.1)
      (Physics|SetSimulatePhysics (Variables|Default|GetStone) true))
    (:then_2
      (Utilities|FlowControl|Delay 3.0)
      (CallFunction|FinishStone)
      (Utilities|FlowControl|Delay 0.2)
      (Actor|DestroyActor))))

(fn ConstructionScript)

(fn HitBird
  (bind _birdbpref (Variables|Default|GetBirdBPRef))
  (bind _result (Math|Integer|IncrementInt (Variables|Default|GetTimesHitBird))
    (:%20%20
      (bind _output_get (Variables|Default|SetTimesHitBird _result))
      (if (> _output_get 1)
        (Utilities|IsValid _birdbpref
          (:Is%20Valid
            (Variables|/Game/Birds/Birds/Bird_MasterBP.Bird_MasterBP_C|SetbGotBonus _birdbpref true)
            (Variables|Default|SetbGotBonus true)
            (bind _result_2 (Math|Integer|IncrementInt (Variables|Default|GetCurrentMultiplier))
              (:%20%20
                (Variables|Default|SetCurrentMultiplier _result_2)
                (CallFunction|DisplayBonusText)))))))))