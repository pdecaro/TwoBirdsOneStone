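; Arcade cabinet actor that serves as an in-world stage for a retro game start menu, with its own camera and screen.
; On BeginPlay it waits, blends the player view to the cabinet camera, then plays turn-on and intro sounds around creating the RetroStartMenu widget in the viewport.
; Separate events drive a timeline that zooms the camera boom in or back, and show or hide the whole cabinet through root visibility.
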(event Custom|HideCabinet
  ;[1 1 1] Hide and Show Stage
  (Rendering|SetVisibility (Variables|Default|GetRoot) false true))

(event Custom|TurnOnScreen
  ;[1 1 1] Turn On Screen
  (Audio|PlaySoundatLocation "/Game/Audio/SoundEffects/Cabinet/Screen_TurnOn_Cue.Screen_TurnOn_Cue" (Transformation|GetWorldLocation (Variables|Default|GetSM_Screen_Panel_01)) "0, 0, 0" 1.0 1.0 0.0 0 0 0)
  (Utilities|FlowControl|Delay 0.75)
  (bind _returnvalue (UserInterface|CreateWidget "/Game/UI/RetroStartMenu.RetroStartMenu_C"))
  (bind _output_get (Variables|Default|SetCurrentWidgetRef _returnvalue))
  (UserInterface|Viewport|AddtoViewport _output_get 0)
  (Audio|PlaySoundatLocation "/Game/Audio/SoundEffects/Cabinet/GameIntro01_Cue.GameIntro01_Cue" (Transformation|GetWorldLocation (Variables|Default|GetSM_Screen_Panel_01)) "0, 0, 0" 1.0 1.0 0.0 0 0 0))

(event Custom|UseCabinetCamera
  ;[1 1 1] Use Cabinet Camera
  (Game|Player|SetViewTargetwithBlend (Game|GetPlayerController 0) self 2.0 "VTBlend_Linear" 1.0 false))

(event Custom|ShowCabinet
  ;[1 1 1] Hide and Show Stage
  (Rendering|SetVisibility (Variables|Default|GetRoot) true true))

(event Custom|ZoomIn
  ;[1 1 1] Camera Zoom
  (bind _smoothzoom (Timeline|Zoom PlayFromStart)
    (:Update
      (Variables|/Script/Engine.SpringArmComponent|SetTargetArmLength (Variables|Default|GetCameraBoom) _smoothzoom))))

(event Custom|ZoomBack
  ;[1 1 1] Camera Zoom
  (bind _smoothzoom (Timeline|Zoom Reverse)
    (:Update
      (Variables|/Script/Engine.SpringArmComponent|SetTargetArmLength (Variables|Default|GetCameraBoom) _smoothzoom))))

(event EventBeginPlay
  ;[1 1 1] Begin Play
  (Utilities|FlowControl|Delay 2.15)
  (CallFunction|UseCabinetCamera)
  (Utilities|FlowControl|Delay 2.2)
  (CallFunction|TurnonScreen))

(fn ConstructionScript)