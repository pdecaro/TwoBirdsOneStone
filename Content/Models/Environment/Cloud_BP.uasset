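; Environment prop of a cloud hung on two cables that wobbles when hit by a stone projectile.
; Construction script lines up the cable pivots, attaches both cable ends and raises the start pivots to CableHeight; BeginPlay re-attaches the ends.
; A hit plays a sound, gated by a DoOnce that resets after a short delay, when a timeline also shifts and yaws the cloud.
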(event OnComponentHit(Cloud)
  (params (HitComponent :type Primitive%20Component%20Object%20Reference) (OtherActor :type Actor%20Object%20Reference) (OtherComp :type Primitive%20Component%20Object%20Reference) (NormalImpulse :type Vector :default "0, 0, 0") (Hit :type Hit%20Result%20Structure%20%28by%20ref%29))
  (Utilities|Casting|CastToStoneProjectile_BP OtherActor)
  (Utilities|FlowControl|Sequence
    (:then_0
      (Utilities|FlowControl|Delay 0.1)
      (CallFunction|CloudDisturbed)
      (goto _label Reset))
    (:then_1
      (Utilities|FlowControl|DoOnce false :!label _label
        (:Completed
          (Audio|PlaySoundatLocation "/Game/Audio/SoundEffects/Impacts/BirdHit01_Cue.BirdHit01_Cue" "0, 0, 0" "0, 0, 0" 0.5 0.75 0.0 0 0 0))))))

(event Custom|CloudDisturbed
  (bind _cloud (Variables|Default|GetCloud))
  (bind (_direction _disturbx _disturbrotz) (Timeline|CloudDistrubedSmooth PlayFromStart)
    (:Update
      (Transformation|SetRelativeLocation _cloud (Math|Vector|MakeVector _disturbx 0.0 0.0) false false)
      (Transformation|SetRelativeRotation _cloud (Math|Rotator|MakeRotator 0.0 0.0 _disturbrotz) false false))))

(event EventBeginPlay
  ;[1 1 1] Begin Play
  (bind _asplayer_bp (Utilities|Casting|CastToPlayerBP (Game|Player|GetPlayerPawn 0)))
  (Variables|Default|SetPlayerBPRef _asplayer_bp)
  (Class|CableComponent|SetAttachEndtoComponent (Variables|Default|GetCable) (Variables|Default|GetCablePivotEnd) "None")
  (Class|CableComponent|SetAttachEndtoComponent (Variables|Default|GetCable1) (Variables|Default|GetCable1PivotEnd) "None"))

(fn ConstructionScript
  (bind _cable1 (Variables|Default|GetCable1))
  (bind _cable1pivotstart (Variables|Default|GetCable1PivotStart))
  (bind _cablepivotstart (Variables|Default|GetCablePivotStart))
  (bind _cable (Variables|Default|GetCable))
  (bind _relativelocation (Variables|/Script/Engine.SceneComponent|GetRelativeLocation _cable1pivotstart))
  (bind _relativelocation_2 (Variables|/Script/Engine.SceneComponent|GetRelativeLocation _cablepivotstart))
  (Utilities|FlowControl|Sequence
    (:then_0
      (Transformation|SetRelativeLocation (Variables|Default|GetCablePivotEnd) (Math|Vector|MakeVector (.x (Variables|/Script/Engine.SceneComponent|GetRelativeLocation (Variables|Default|GetCablePivotStart))) 0.0 0.0) false false)
      (Transformation|SetRelativeLocation (Variables|Default|GetCable1PivotEnd) (Math|Vector|MakeVector (.x (Variables|/Script/Engine.SceneComponent|GetRelativeLocation (Variables|Default|GetCable1PivotStart))) 0.0 0.0) false false))
    (:then_1
      (Transformation|AttachComponentToComponent _cable (Variables|Default|GetCablePivotStart) "None" "SnapToTarget" "SnapToTarget" "SnapToTarget" true)
      (Transformation|AttachComponentToComponent _cable1 (Variables|Default|GetCable1PivotStart) "None" "SnapToTarget" "SnapToTarget" "SnapToTarget" true))
    (:then_2
      (Class|CableComponent|SetAttachEndtoComponent _cable (Variables|Default|GetCablePivotEnd) "None")
      (Class|CableComponent|SetAttachEndtoComponent _cable1 (Variables|Default|GetCable1PivotEnd) "None"))
    (:then_3
      (Transformation|SetRelativeLocation _cable1pivotstart (Math|Vector|MakeVector (.x _relativelocation) (.y _relativelocation) (Variables|Default|GetCableHeight)) false false)
      (Transformation|SetRelativeLocation _cablepivotstart (Math|Vector|MakeVector (.x _relativelocation_2) (.y _relativelocation_2) (Variables|Default|GetCableHeight)) false false))))